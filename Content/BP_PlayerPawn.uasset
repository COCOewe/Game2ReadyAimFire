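; Player pawn blueprint that lets the player spawn, aim and fire a cannon through Enhanced Input.
; BeginPlay adds the player mapping context.
; The spawn input toggles an equipped flag, either spawning a cannon actor at the right hand's transform or destroying it.
; Aim input rotates the cannon's root in pitch and yaw, and fire input calls the cannon's Fire.
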(event `EnhancedInput|/Game/IA_CannonFire`
  (params (ActionValue :type Boolean) (ElapsedSeconds :type "Float (double-precision)") (TriggeredSeconds :type "Float (double-precision)") (InputAction :type "InputAction Object Reference" :default "/Game/IA_CannonFire.IA_CannonFire"))
  (:`Started`
    (`/Game/BP_CannonActor.Fire` (`self.BPcannon`))))

(event `EnhancedInput|/Game/IA_CannonAim`
  (params (ActionValue :type "Vector2D Structure") (ElapsedSeconds :type "Float (double-precision)") (TriggeredSeconds :type "Float (double-precision)") (InputAction :type "InputAction Object Reference" :default "/Game/IA_CannonAim.IA_CannonAim"))
  (bind _bpcannon (`self.BPcannon`))
  (:`Triggered`
    (`/Engine/EditorBlueprintResources/StandardMacros.IsValid` _bpcannon
      (:`Is Valid`
        (`SceneComponent.K2_AddLocalRotation` (`Actor.RootComponent` _bpcannon) (`KismetMathLibrary.MakeRotator` 0.0 ActionValue_Y ActionValue_X) false false)))))

(event `EnhancedInput|/Game/IA_CannonSpawn`
  (params (ActionValue :type Boolean) (ElapsedSeconds :type "Float (double-precision)") (TriggeredSeconds :type "Float (double-precision)") (InputAction :type "InputAction Object Reference" :default "/Game/IA_CannonSpawn.IA_CannonSpawn"))
  (:`Started`
    (bind _output_get (set `self.IsEquipped` (not (`self.IsEquipped`))))
    (if _output_get
      (`KismetSystemLibrary.PrintString` "Hello")
      (bind _returnvalue (`|SpawnActorFromClass` "/Game/BP_CannonActor.BP_CannonActor_C" (`SceneComponent.K2_GetComponentToWorld` (`self.RightHand`)) "Undefined" "MultiplyWithRoot" null null))
      (set `self.BPcannon` _returnvalue)
      (else
        (`self.K2_DestroyActor` (`self.BPcannon`))))))

(event `self.ReceiveBeginPlay`
  (bind _returnvalue (pcsubsystem `EnhancedInputLocalPlayerSubsystem` (`GameplayStatics.GetPlayerController` 0)))
  (`/Engine/EditorBlueprintResources/StandardMacros.IsValid` _returnvalue
    (:`Is Valid`
      (`EnhancedInputSubsystemInterface.AddMappingContext` _returnvalue "/Game/IMC_PlayerMapping.IMC_PlayerMapping" 0 (struct)))))

(fn `UserConstructionScript`)